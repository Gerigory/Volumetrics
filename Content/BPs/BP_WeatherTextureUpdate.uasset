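; BP_WeatherTextureUpdate renders weather textures by drawing materials into render targets.
; Draw fills the coverage, cloud type, precipitation and composition targets in that order, each from its own material.
; Draw runs every frame while the Tick flag is set, and a separate Clear event resets only the coverage target to black.
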(event `self.ReceiveTick`
  (params (DeltaSeconds :type "Float (single-precision)"))
  (if (`self.Tick`)
    (`self.Draw`)))

(event `Clear`
  (`KismetRenderingLibrary.ClearRenderTarget2D` (`self.CoverageRT`)))

(event `Draw`
  (`KismetRenderingLibrary.DrawMaterialToRenderTarget` (`self.CoverageRT`) (`self.CoverageMtl`))
  (`KismetRenderingLibrary.DrawMaterialToRenderTarget` (`self.CloudTypeRT`) (`self.CloudTypeMtl`))
  (`KismetRenderingLibrary.DrawMaterialToRenderTarget` (`self.PrecipitationRT`) (`self.PrecipitationMtl`))
  (`KismetRenderingLibrary.DrawMaterialToRenderTarget` (`self.CompositionRT`) (`self.CompositionMtl`)))

(fn `UserConstructionScript`)