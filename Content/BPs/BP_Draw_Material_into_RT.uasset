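; BP_Draw_Material_into_RT bakes PW, Worley and Curl materials, apparently procedural noise, into render targets.
; The Draw event renders each of the three materials into its own render target with DrawMaterialToRenderTarget.
; A Tick flag optionally repeats the draw every frame.
; A separate Clear event resets only the PW render target to opaque black.
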(event `self.ReceiveTick`
  (params (DeltaSeconds :type "Float (single-precision)"))
  (if (`self.Tick`)
    (`self.Draw`)))

(event `Clear`
  (`KismetRenderingLibrary.ClearRenderTarget2D` (`self.PWRender Target`)))

(event `Draw`
  (`KismetRenderingLibrary.DrawMaterialToRenderTarget` (`self.PWRender Target`) (`self.PWMaterial`))
  (`KismetRenderingLibrary.DrawMaterialToRenderTarget` (`self.WorleyRender Target`) (`self.WorleyMaterial`))
  (`KismetRenderingLibrary.DrawMaterialToRenderTarget` (`self.CurlRender Target`) (`self.CurlMaterial`)))

(fn `UserConstructionScript`)