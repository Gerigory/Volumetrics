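; Demo actor that drives what appears to be a raymarched volumetric cloud material on a sky sphere, despite its WaterMarching name.
; The construction script creates a dynamic material instance, applies it to EditorSkySphere and toggles the dome's visibility.
; It then pushes cloud layer, earth scale, march step, weather, detail, speed and color variables into the material, packing several into vector parameters.
; The event graph has no active logic.
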(fn `UserConstructionScript`
  (bind _mid (`self.MID`))
  (bind _mid_2 (`self.MID`))
  (bind _cloud_altitude_km (`self.Cloud Altitude Km`))
  (`/Volumetrics/Tools/BlueprintLibraries/VolumetricsBPLIbrary.Create and Assign MID` (`self.MID`) (`self.Material`))
  (`PrimitiveComponent.SetMaterial` (`self.EditorSkySphere`) 0 (`self.MID`))
  (`SceneComponent.SetVisibility` (`self.EditorSkySphere`) (`self.Show Sky Dome`) false)
  (`MaterialInstanceDynamic.SetVectorParameterValue` _mid_2 "CloudMinMax" (make `LinearColor` _cloud_altitude_km (+ _cloud_altitude_km (`self.Cloud Layer Thickness Km`)) (`self.Cloud Tile Size Km`) (`self.CoverageScale`)))
  (`MaterialInstanceDynamic.SetScalarParameterValue` _mid_2 "EarthScale" (`self.EarthRadiusScale`))
  (`MaterialInstanceDynamic.SetScalarParameterValue` _mid_2 "StepSize" (`self.Stepsize`))
  (`MaterialInstanceDynamic.SetScalarParameterValue` _mid_2 "MaxSteps" (`self.MaxSteps`))
  (`MaterialInstanceDynamic.SetScalarParameterValue` _mid_2 "LightStepSize" (`self.LightStepSize`))
  (`MaterialInstanceDynamic.SetScalarParameterValue` _mid_2 "VolumeResolution" (`self.VolumeResolution`))
  (`MaterialInstanceDynamic.SetVectorParameterValue` _mid "WeatherParams" (make `LinearColor` (`self.WeatherScale`) (/ 1.0 (`self.DensityScale`))))
  (`MaterialInstanceDynamic.SetVectorParameterValue` _mid "CloudScaleParams" (make `LinearColor` (`self.LowFreqDetailScale`) (`self.HighFreqDetailScale`) (`self.DebugVisibility`) (`self.HFScale`)))
  (`MaterialInstanceDynamic.SetVectorParameterValue` _mid "CloudSpeedParams" (`self.CloudSpeed`))
  (`MaterialInstanceDynamic.SetVectorParameterValue` _mid "BrightColor" (`self.BrightColor`))
  (`MaterialInstanceDynamic.SetVectorParameterValue` _mid "DarkColor" (`self.DarkColor`)))